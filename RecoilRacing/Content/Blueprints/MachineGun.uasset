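; MachineGun is a gun Blueprint whose shots push the player character by launching it along the given direction, scaled by Force.
; Tick counts down a timer that gates CanShoot.
; Shoot plays the gun sound at the player pawn, restarts the timer and multiplies Cooldown by a decay factor, so the delay changes with each shot.
; ResetCooldown restores the base cooldown.
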(event EventBeginPlay)

(event EventTick
  (params (DeltaSeconds :type Float%20%28single-precision%29))
  (if (> (Variables|Default|GetTimer) 0.0)
    (Variables|Default|SetTimer (- (Variables|Default|GetTimer) DeltaSeconds))
    (Variables|Default|SetCanShoot false)
    (else
      (Variables|Default|SetCanShoot true))))

(fn Shoot
  (params (Direction :type Vector))
  (if (Variables|Default|GetCanShoot)
    (Audio|PlaySoundatLocation (Variables|Default|GetGunSound) (Transformation|GetActorLocation (Game|Player|GetPlayerPawn 0)) "0, 0, 0" 1.0 1.0 0.0 0 0 0 0)
    (Variables|Default|SetTimer (Variables|Default|GetCooldown))
    (Variables|Default|SetCooldown (* (Variables|Default|GetCooldown) (Variables|Default|GetCooldownDecay)))
    (Character|LaunchCharacter (Game|GetPlayerCharacter 0) (* Direction (Variables|Default|GetForce)) false false)))

(fn ResetCooldown
  (Variables|Default|SetCooldown (Variables|Default|GetBaseCooldown)))