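; RecoilController is a controller that respawns the player's pawn at an active checkpoint when R is pressed, a key binding marked as temporary.
; FindRespawnPoint scans the RecoilGameState checkpoints, selects an active one and returns its location plus SpawnOffset.
; The selection compares checkpoint indices but stores array indices, and a note admits order is not guaranteed.
; On success, the pawn teleports there with zero rotation and zero velocity.
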(event EventBeginPlay)

(event EventTick
  (params (DeltaSeconds :type Float%20%28single-precision%29)))

(event Input|KeyboardEvents|R
  (params (Key :type Key%20Structure :default "None"))
  (bind _returnvalue (Pawn|GetControlledPawn))
  ;[1 1 1] This is temporary. It should be bound to a proper input action.
  (:Pressed
    (bind (_bsuccess _respawnpoint) (CallFunction|FindRespawnPoint))
    (if _bsuccess
      (Transformation|Teleport _returnvalue _respawnpoint "0, 0, 0")
      (Variables|/Script/Engine.MovementComponent|SetVelocity (Pawn|GetMovementComponent _returnvalue) "0, 0, 0"))))

(fn ConstructionScript)

(fn FindRespawnPoint
  ;[1 1 1] Logic needs cleaned. Order cannot be guaranteed, just respawns at first active point. Need to determine if there can be more than one.
  (bind _asrecoil_game_state (Utilities|Casting|CastToRecoilGameState (Game|GetGameState)))
  (for (_array_element _array_index) (Variables|/Game/Blueprints/RecoilGameState.RecoilGameState_C|GetCheckpoints _asrecoil_game_state)
    (bind _returnvalue (Class|CheckPoint|GetCheckPointIndex _array_element))
    (bind _returnvalue_2 (Class|CheckPoint|IsActive _array_element))
    (if (and _returnvalue_2 (> _returnvalue (LocalVariables|GetSelectedCheckpointIndex)))
      (LocalVariables|SetSelectedCheckpointIndex _array_index)))
  (if (>= (LocalVariables|GetSelectedCheckpointIndex) 0)
    (LocalVariables|SetbPointFound true)
    (LocalVariables|SetPoint (+ (Transformation|GetActorLocation (Utilities|Array|Get(acopy) (Variables|/Game/Blueprints/RecoilGameState.RecoilGameState_C|GetCheckpoints _asrecoil_game_state) (LocalVariables|GetSelectedCheckpointIndex))) (LocalVariables|GetSpawnOffset))))
  (return (LocalVariables|GetbPointFound) (LocalVariables|GetPoint)))