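; Game state for Recoil that provides checkpoint respawn locations and keeps the persistent best completion time.
; On BeginPlay it gathers all checkpoint actors and asynchronously loads the "TheBest" save slot.
; FindRespawnPoint selects the highest-index active checkpoint, never moving backwards, though actor array order is not guaranteed.
; CompleteGame saves a new time when no valid record exists or it beats the loaded one, returning whether it saved.
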(event EventBeginPlay
  (bind _outactors (Actor|GetAllActorsOfClass "/Game/Objects/BP_CheckPoint.BP_CheckPoint_C"))
  (Variables|Default|SetCheckpoints _outactors)
  (bind (_savegame _bsuccess) (|AsyncLoadGamefromSlot "TheBest")
    (:Completed
      (if _bsuccess
        (bind _asrecoil_save_game (Utilities|Casting|CastToRecoilSaveGame _savegame))
        (Variables|Default|SetSaveGame _asrecoil_save_game)))))

(event EventTick
  (params (DeltaSeconds :type Float%20%28single-precision%29)))

(fn ConstructionScript)

(fn FindRespawnPoint
  (bind _checkpoints (Variables|Default|GetCheckpoints))
  ;[1 1 1] Logic needs cleaned. Order cannot be guaranteed, just respawns at first active point. Need to determine if there can be more than one.
  (for (_array_element _array_index) _checkpoints
    (bind _returnvalue (Class|CheckPoint|IsActive _array_element))
    (if (and _returnvalue (> _array_index (LocalVariables|GetSelectedCheckpointIndex)))
      (LocalVariables|SetSelectedCheckpointIndex _array_index)))
  (if (>= (LocalVariables|GetSelectedCheckpointIndex) 0)
    (LocalVariables|SetbPointFound true)
    (LocalVariables|SetPoint (Transformation|GetActorLocation (Utilities|Array|Get(acopy) _checkpoints (LocalVariables|GetSelectedCheckpointIndex)))))
  (return (LocalVariables|GetbPointFound) (LocalVariables|GetPoint)))

(fn CompleteGame
  (params (NewTime :type Timespan%20Structure))
  (bind _savegame (Variables|Default|GetSaveGame))
  (Utilities|IsValid _savegame
    (:Is%20Valid
      (if (or (< NewTime (Variables|/Game/Blueprints/RecoilSaveGame.RecoilSaveGame_C|GetBestTime _savegame)) (<= (Variables|/Game/Blueprints/RecoilSaveGame.RecoilSaveGame_C|GetBestTime _savegame) (Class|KismetMathLibrary|TimespanZeroValue)))
        _
        (else
          (return false))))
    (:Is%20Not%20Valid
      _))
  (bind _returnvalue (SaveGame|CreateSaveGameObject "/Game/Blueprints/RecoilSaveGame.RecoilSaveGame_C"))
  (Variables|/Game/Blueprints/RecoilSaveGame.RecoilSaveGame_C|SetBestTime _returnvalue NewTime)
  (SaveGame|SaveGametoSlot _returnvalue "TheBest")
  (return true))