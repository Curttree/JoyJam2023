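; Animation notify that plays surface-specific footstep sounds for the animated mesh's owner.
; On notify, it line-traces on the Visibility channel a short distance straight down from the owner's location and reads the hit's surface type.
; Grass, Stone and Water each play their own sound cue at the impact location, while any other surface or a missed trace plays nothing.
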(fn GetNotifyName
  (return ""))

(fn ReceivedNotify
  (params (MeshComp :type Skeletal%20Mesh%20Component%20Object%20Reference) (Animation :type Anim%20Sequence%20Base%20Object%20Reference) (EventReference :type Anim%20Notify%20Event%20Reference%20Structure%20%28by%20ref%29))
  (bind _returnvalue (Components|GetOwner MeshComp))
  (bind _returnvalue_2 (Transformation|GetActorLocation _returnvalue))
  (bind (_outhit _returnvalue_3) (Collision|LineTraceByChannel _returnvalue_2 (- _returnvalue_2 "0,0,150.000000") "TraceTypeQuery1" false 0 "None"))
  (if _returnvalue_3
    (switch Utilities|FlowControl|Switch|SwitchonEPhysicalSurface (Collision|GetSurfaceType _outhit)
      (:SurfaceType_Default
        (return false))
      (:SurfaceType1
        (Audio|PlaySoundatLocation "/Game/Sounds/SoundFX/Cues/Locomotion/Steps/Grass/CUE_Grass_footsteps.CUE_Grass_footsteps" (.Location (Collision|BreakHitResult _outhit)) "0, 0, 0" 1.0 1.0 0.0 0 0 0 0))
      (:SurfaceType2
        (Audio|PlaySoundatLocation "/Game/Sounds/SoundFX/Cues/Locomotion/Steps/Stone/CUE_StoneFootsteps.CUE_StoneFootsteps" (.Location (Collision|BreakHitResult _outhit)) "0, 0, 0" 1.0 1.0 0.0 0 0 0 0))
      (:SurfaceType3
        (Audio|PlaySoundatLocation "/Game/Sounds/SoundFX/Cues/Locomotion/Steps/Water/CUE_Water_footstep_Cue.CUE_Water_footstep_Cue" (.Location (Collision|BreakHitResult _outhit)) "0, 0, 0" 1.0 1.0 0.0 0 0 0 0)))))