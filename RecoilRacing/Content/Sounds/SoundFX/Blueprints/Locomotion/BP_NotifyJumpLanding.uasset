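; Animation notify that plays a jump landing sound matched to the surface under the character.
; On notify, it line traces a short distance down from the owning actor on the Visibility channel.
; The hit's physical surface type selects a grass, stone or water landing cue, played at the impact point; other surfaces play nothing.
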(fn GetNotifyName
  (return ""))

(fn ReceivedNotify
  (params (MeshComp :type Skeletal%20Mesh%20Component%20Object%20Reference) (Animation :type Anim%20Sequence%20Base%20Object%20Reference) (EventReference :type Anim%20Notify%20Event%20Reference%20Structure%20%28by%20ref%29))
  (bind _returnvalue (Components|GetOwner MeshComp))
  (bind _returnvalue_2 (Transformation|GetActorLocation _returnvalue))
  (bind (_outhit _returnvalue_3) (Collision|LineTraceByChannel _returnvalue_2 (- _returnvalue_2 "0,0,150.000000") "TraceTypeQuery1" false 0 "None"))
  (if _returnvalue_3
    (switch Utilities|FlowControl|Switch|SwitchonEPhysicalSurface (Collision|GetSurfaceType _outhit)
      (:SurfaceType_Default
        (return false))
      (:SurfaceType1
        (Audio|PlaySoundatLocation "/Game/Sounds/SoundFX/Cues/Locomotion/Jump/Landing/Grass/Grass_JumpLanding_Cue.Grass_JumpLanding_Cue" (.Location (Collision|BreakHitResult _outhit)) "0, 0, 0" 1.0 1.0 0.0 0 0 0 0))
      (:SurfaceType2
        (Audio|PlaySoundatLocation "/Game/Sounds/SoundFX/Cues/Locomotion/Jump/Landing/Stone/CUE_Jump_Land_Stone_Cue.CUE_Jump_Land_Stone_Cue" (.Location (Collision|BreakHitResult _outhit)) "0, 0, 0" 1.0 1.0 0.0 0 0 0 0))
      (:SurfaceType3
        (Audio|PlaySoundatLocation "/Game/Sounds/SoundFX/Cues/Locomotion/Jump/Landing/Water/JumpLand_Water_Cue.JumpLand_Water_Cue" (.Location (Collision|BreakHitResult _outhit)) "0, 0, 0" 1.0 1.0 0.0 0 0 0 0)))))