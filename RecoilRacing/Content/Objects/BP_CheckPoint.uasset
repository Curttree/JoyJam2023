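; BP_CheckPoint is a checkpoint flag that changes colour and plays a sound when activated.
; On BeginPlay it creates a dynamic material instance on the Flag and sets its FlagColour parameter to the inactive colour.
; An actor overlap calls TryActivate, whose logic is not in this graph; on success the flag switches to the active colour and a midway-gate sound spawns at the actor's location.
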(event EventBeginPlay
  (bind _returnvalue (Rendering|Material|CreateDynamicMaterialInstance (Variables|Default|GetFlag) 0 0 "None" :!class /Script/Engine.PrimitiveComponent))
  (bind _output_get (Variables|Default|SetFlagColour _returnvalue))
  (Rendering|Material|SetVectorParameterValue _output_get "FlagColour" (Variables|Default|GetInactiveColour) :!class /Script/Engine.MaterialInstanceDynamic))

(event Collision|EventActorBeginOverlap
  (params (OtherActor :type Actor%20Object%20Reference))
  (bind _returnvalue (Class|CheckPoint|TryActivate))
  (if _returnvalue
    (Rendering|Material|SetVectorParameterValue (Variables|Default|GetFlagColour) "FlagColour" (Variables|Default|GetActiveColour) :!class /Script/Engine.MaterialInstanceDynamic)
    (Audio|SpawnSoundatLocation "/Game/Sounds/smw_midway_gate.smw_midway_gate" (Transformation|GetActorLocation) "0, 0, 0" 1.0 1.0 0.0 0 0)))

(event EventTick
  (params (DeltaSeconds :type Float%20%28single-precision%29)))

(fn ConstructionScript)