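; BP_Ghost is a ghost pawn that replays a recorded list of positions supplied through SetGhostData.
; Tick advances through the timed targets, setting FloatingPawnMovement speed from distance over remaining time and having BP_GhostController move it to each point.
; When no target remains, it hides itself and spawns a despawn effect.
; It starts at the player's location, and ClearGhostData deletes the "TheBest" save slot.
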(event Custom|SetGhostData
  (params (InGhostData :type Array%20of%20Vector%204%20Structures))
  (Variables|Default|SetGhostPositions InGhostData)
  (Rendering|SetActorHiddenInGame false))

(event EventBeginPlay
  (Transformation|SetActorLocation (Transformation|GetActorLocation (Game|Player|GetPlayerPawn 0)) false true))

(event Collision|EventActorBeginOverlap
  (params (OtherActor :type Actor%20Object%20Reference)))

(event EventTick
  (params (DeltaSeconds :type Float%20%28single-precision%29))
  (if (Math|Boolean|ANDBoolean (>= (Utilities|Time|GetTimeSeconds) (Variables|Default|GetNextTargetUpdateTime)) (not (Variables|Default|GetbFinishedMoving)) (> (Utilities|Array|Length (Variables|Default|GetGhostPositions)) 0))
    (bind _returnvalue (Class|Ghost|TryIncrement))
    (if _returnvalue
      (Variables|/Script/Engine.FloatingPawnMovement|SetMaxSpeed (Variables|Default|GetFloatingPawnMovement) (Math|Float|SafeDivide (Math|Vector|Distance(Vector) (Transformation|GetActorLocation) (Variables|Default|GetNextTargetPosition)) (- (Variables|Default|GetNextTargetUpdateTime) (Utilities|Time|GetTimeSeconds))))
      (bind _asbp_ghost_controller (Utilities|Casting|CastToBP_GhostController (Pawn|GetController)))
      (Default|MovetoPoint _asbp_ghost_controller (Variables|Default|GetNextTargetPosition))
      (else
        (Variables|Default|SetbFinishedMoving true)
        (Rendering|SetActorHiddenInGame true)
        (Niagara|SpawnSystematLocation "/Game/Objects/GhostDespawn.GhostDespawn" (Transformation|GetWorldLocation (Variables|Default|GetSphere)))))))

(fn ConstructionScript)

(fn ClearGhostData
  (SaveGame|DeleteGameinSlot "TheBest"))